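; BP_platform is a player-controlled paddle for a ball game that shifts sideways along Y by a fixed, unswept step from the MoveRight axis.
; Positive input also calls Endgame on the BP_platform actors found in the level.
; Endgame decrements MaxLifes when no BP_ball actors remain, then creates and displays Game_widget once lives run out.
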(event `InputAxis|MoveRight`
  (params (AxisValue :type "Float (single-precision)"))
  (if (< AxisValue 0.0)
    (`self.K2_AddActorWorldOffset` (0.0 -50.0 0.0))))

(event `InputAxis|MoveRight`
  (params (AxisValue :type "Float (single-precision)"))
  (if (> AxisValue 0.0)
    (`self.K2_AddActorWorldOffset` (0.0 50.0 0.0))
    (bind _outactors (`GameplayStatics.GetAllActorsOfClass` "BP_platform_C"))
    (`self.endgame` _outactors)))

(event `endgame`
  (bind _outactors (`GameplayStatics.GetAllActorsOfClass` "/Game/MyLogic/task_1/BP_ball.BP_ball_C"))
  (if (not (> (`KismetArrayLibrary.Array_Length` _outactors) 0))
    (bind _result (`/Engine/EditorBlueprintResources/StandardMacros.DecrementInt` (`self.MaxLifes`))
      (:`  `
        (if (not (> _result 0))
          (bind _returnvalue (`|CreateWidget` "/Game/MyLogic/task_1/Game_widget.Game_widget_C"))
          (`UserWidget.AddToViewport` _returnvalue 0))))))

(fn `UserConstructionScript`)